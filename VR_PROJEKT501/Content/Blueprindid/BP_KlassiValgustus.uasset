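; Classroom lighting Blueprint that lets the player switch the front lights on and off from inside an interaction zone.
; Zone overlap enables or disables player input and toggles the F and G key help texts.
; Pressing F toggles the visibility of the front point lights.
; The rear-light section holds only disconnected toggle and delay nodes, with no G key handler.
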(event OnComponentBeginOverlap(ReageerimisTzoon)
  (params (OverlappedComponent :type Primitive%20Component%20Object%20Reference) (OtherActor :type Actor%20Object%20Reference) (OtherComp :type Primitive%20Component%20Object%20Reference) (OtherBodyIndex :type Integer) (bFromSweep :type Boolean) (SweepResult :type Hit%20Result%20Structure%20%28by%20ref%29))
  ;[1 0.1838 0] Reageerimistzoonis olemine. Kuvatakse abitekst ja reageeritakse klahvivajutustele.
  (Input|EnableInput (Game|GetPlayerController 0))
  (Rendering|ToggleVisibility (Variables|Default|GetAbiTekst%20F%20klahv) false))

(event OnComponentEndOverlap(ReageerimisTzoon)
  (params (OverlappedComponent :type Primitive%20Component%20Object%20Reference) (OtherActor :type Actor%20Object%20Reference) (OtherComp :type Primitive%20Component%20Object%20Reference) (OtherBodyIndex :type Integer))
  ;[1 0.1838 0] Reageerimistzoonis olemine. Kuvatakse abitekst ja reageeritakse klahvivajutustele.
  (Input|DisableInput (Game|GetPlayerController 0))
  (Rendering|ToggleVisibility (Variables|Default|GetAbiTekst%20F%20klahv) false))

(event Input|KeyboardEvents|F
  (params (Key :type Key%20Structure))
  ;[0 0.4127 1] Eesmised valgustid
  (:Pressed
    (Rendering|ToggleVisibility (Variables|Default|GetPointLight) false)))

(event Input|KeyboardEvents|G
  (params (Key :type Key%20Structure))
  ;[0 0.0581 1] Tagumised valgustid
)

(fn ConstructionScript)