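; Door Blueprint ("Uks") that swings open when anything starts overlapping its Trigger component and swings back when an overlap ends.
; Overlap events play or reverse a timeline whose track lerps the Uks component's relative yaw from DoorStart to 90 degrees beyond it.
; The construction script sets DoorStart from the actor's world yaw, though the timeline applies it as a relative rotation.
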(event OnComponentEndOverlap(Trigger)
  (params (OverlappedComponent :type Primitive%20Component%20Object%20Reference) (OtherActor :type Actor%20Object%20Reference) (OtherComp :type Primitive%20Component%20Object%20Reference) (OtherBodyIndex :type Integer))
  (bind _doorstart (Variables|DoorSetup|GetDoorStart))
  ;[1 1 1] UKS
  (bind _newtrack_0 (Timeline|Timeline_0 Reverse)
    (:Update
      (Transformation|SetRelativeRotation (Variables|Default|GetUks) (Math|Rotator|MakeRotator 0.0 0.0 (Math|Float|Lerp _doorstart (+ _doorstart 9e+01) _newtrack_0)) false false))))

(event OnComponentBeginOverlap(Trigger)
  (params (OverlappedComponent :type Primitive%20Component%20Object%20Reference) (OtherActor :type Actor%20Object%20Reference) (OtherComp :type Primitive%20Component%20Object%20Reference) (OtherBodyIndex :type Integer) (bFromSweep :type Boolean) (SweepResult :type Hit%20Result%20Structure%20%28by%20ref%29))
  (bind _doorstart (Variables|DoorSetup|GetDoorStart))
  ;[1 1 1] UKS
  (bind _newtrack_0 (Timeline|Timeline_0 Play)
    (:Update
      (Transformation|SetRelativeRotation (Variables|Default|GetUks) (Math|Rotator|MakeRotator 0.0 0.0 (Math|Float|Lerp _doorstart (+ _doorstart 9e+01) _newtrack_0)) false false))))

(fn ConstructionScript
  (Variables|DoorSetup|SetDoorStart (.yaw (Transformation|GetActorRotation (Components|GetOwner (Variables|Default|GetUks))))))